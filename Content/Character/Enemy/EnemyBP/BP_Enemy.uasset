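; BP_Enemy is an enemy that damages the player character on contact.
; When its Box component begins overlapping a BP_Character, it subtracts EnemyDamage directly from that character's Health.
; If Health falls to ZeroHealth or below, the enemy itself creates the WB_GameOver widget, adds it to the viewport and shows the mouse cursor.
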(event OnComponentBeginOverlap(Box)
  (params (OverlappedComponent :type Primitive%20Component%20Object%20Reference) (OtherActor :type Actor%20Object%20Reference) (OtherComp :type Primitive%20Component%20Object%20Reference) (OtherBodyIndex :type Integer) (bFromSweep :type Boolean) (SweepResult :type Hit%20Result%20Structure%20%28by%20ref%29))
  (bind _asbp_character (Utilities|Casting|CastToBP_Character OtherActor))
  (Variables|/Game/Main/BP_Character.BP_Character_C|SetHealth _asbp_character (- (Variables|/Game/Main/BP_Character.BP_Character_C|GetHealth _asbp_character) (Variables|Default|GetEnemyDamage)))
  (if (<= (Variables|/Game/Main/BP_Character.BP_Character_C|GetHealth _asbp_character) (Variables|/Game/Main/BP_Character.BP_Character_C|GetZeroHealth _asbp_character))
    (bind _returnvalue (UserInterface|CreateWidget "/Game/Widget/WB_GameOver.WB_GameOver_C"))
    (UserInterface|Viewport|AddtoViewport _returnvalue 0)
    (Variables|/Script/Engine.PlayerController|SetbShowMouseCursor (Game|GetPlayerController 0) true)))

(event EventBeginPlay)

(event EventTick
  (params (DeltaSeconds :type Float%20%28single-precision%29)))

(fn ConstructionScript)